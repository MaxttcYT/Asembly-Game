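; First-person player character for a Satisfactory-style building game, handling build placement, deconstruction, interaction, sprinting, pausing and health.
; Camera line traces drive looping timers that move the pending A_Builds hologram or highlight a deletion target, while scroll and confirm inputs adjust, place or destroy it.
; Damage, including velocity-based fall damage, updates the controller's health bar, and death shows a widget and requests a GameMode respawn.
; Snow effect activates December 1–24.
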(event Custom|StartSprinting
  (Variables|/Script/Engine.CharacterMovementComponent|SetMaxWalkSpeed (Variables|Character|GetCharacterMovement) 1.5e+03))

(event Custom|CheckCustomDateEvents
  (bind _returnvalue (Math|DateTime|Now))
  (bind _snow (Variables|Default|GetSnow))
  (bind (_year _month _day) (Math|DateTime|BreakDateTime _returnvalue))
  (if (and (== _month 12) (Math|Integer|InRange(Integer) _day 1 24))
    (Components|Activation|Activate _snow false)
    (else
      (Components|Activation|Deactivate _snow))))

(event Custom|StopSprinting
  (Variables|/Script/Engine.CharacterMovementComponent|SetMaxWalkSpeed (Variables|Character|GetCharacterMovement) 6e+02))

(event Custom|Falling
  (bind _returnvalue (Game|GetPlayerCharacter 0))
  (bind _returnvalue_2 (Transformation|GetVelocity _returnvalue))
  (bind _returnvalue_3 (* (.z _returnvalue_2) -1.0))
  (if (AI|Components|NavMovement|IsFalling (Variables|Character|GetCharacterMovement))
    (if (> _returnvalue_3 9e+02)
      (bind _output_get (Variables|Default|SetFallDamage (Math|Conversions|ToFloat(Integer) (Math|Float|Round (Math|Float|Power (/ (/ _returnvalue_3 5e+01) 5.0) (+ (/ _returnvalue_3 3e+03) 2.0))))))
      (Game|Damage|ApplyDamage self _output_get 0 0 "/Script/Engine.DamageType"))))

(event Custom|ConfirmPlacement
  (Variables|Default|GetItemToBuild
    (:then
      (CallFunction|PlaceBuild))
    (:else
      (bind _itemtodelete (Variables|Default|GetItemToDelete)
        (:then
          (Default|DestroyBuild _itemtodelete))
        (:else)))))

(event Custom|scrollBuild
  (params (InputPin :type Float%20%28double-precision%29))
  (bind _itemtobuild (Variables|Default|GetItemToBuild)
    (:then
      (if (Variables|Default|GetIsCtrlDown)
        (Default|ScrollBuildCustom _itemtobuild InputPin)
        (else
          (Default|ScrollBuild _itemtobuild InputPin))))
    (:else)))

(event Input|EnhancedActionEvents|EnhancedInputActionIA_Scroll
  (params (ActionValue :type Float%20%28double-precision%29) (ElapsedSeconds :type Float%20%28double-precision%29) (TriggeredSeconds :type Float%20%28double-precision%29) (InputAction :type Input%20Action%20Object%20Reference :default "/Game/Satisfactory/Blueprints/Inputs/IA_Scroll.IA_Scroll"))
  (:Triggered
    (CallFunction|ScrollBuild ActionValue)
    (bind _itemtobuild (Variables|Default|GetItemToBuild)
      (:then
        (if (Variables|Default|GetIsCtrlDown)
          (Default|ScrollBuildCustom _itemtobuild ActionValue)
          (else
            (Default|ScrollBuild _itemtobuild ActionValue))))
      (:else))))

(event Input|EnhancedActionEvents|EnhancedInputActionIA_Confrm
  (params (ActionValue :type Boolean) (ElapsedSeconds :type Float%20%28double-precision%29) (TriggeredSeconds :type Float%20%28double-precision%29) (InputAction :type Input%20Action%20Object%20Reference :default "/Game/Satisfactory/Blueprints/Inputs/IA_Confrm.IA_Confrm"))
  (:Started
    (CallFunction|ConfirmPlacement)
    (Variables|Default|GetItemToBuild
      (:then
        (CallFunction|PlaceBuild))
      (:else
        (bind _itemtodelete (Variables|Default|GetItemToDelete)
          (:then
            (Default|DestroyBuild _itemtodelete))
          (:else))))))

(event Input|EnhancedActionEvents|EnhancedInputActionIA_Deconstruct
  (params (ActionValue :type Boolean) (ElapsedSeconds :type Float%20%28double-precision%29) (TriggeredSeconds :type Float%20%28double-precision%29) (InputAction :type Input%20Action%20Object%20Reference :default "/Game/Satisfactory/Blueprints/Inputs/IA_Deconstruct.IA_Deconstruct"))
  (:Started
    (if (Utilities|Time|IsValidTimerHandle (Variables|Default|GetDeleteBuild))
      (bind _itemtodelete (Variables|Default|GetItemToDelete)
        (:then
          (Default|SetAllMaterials _itemtodelete 0 true)
          (Variables|Default|SetItemToDelete 0))
        (:else
          _))
      (Utilities|Time|ClearandInvalidateTimerbyHandle (Variables|Default|GetDeleteBuild))
      (else
        (Variables|Default|GetItemToBuild
          (:then
            (CallFunction|CancleBuild))
          (:else
            _))
        (bind _returnvalue (Utilities|Time|SetTimerbyFunctionName 0 "DeterminDelete" 0.05 true))
        (Variables|Default|SetDeleteBuild _returnvalue)))))

(event Input|EnhancedActionEvents|EnhancedInputActionIA_Object1
  (params (ActionValue :type Boolean) (ElapsedSeconds :type Float%20%28double-precision%29) (TriggeredSeconds :type Float%20%28double-precision%29) (InputAction :type Input%20Action%20Object%20Reference :default "/Game/Satisfactory/Blueprints/Inputs/IA_Object1.IA_Object1"))
  (:Started
    (CallFunction|SpawnBuild "/Game/Satisfactory/Blueprints/Buildings/A_Builds_Support.A_Builds_Support_C")))

(event Input|EnhancedActionEvents|EnhancedInputActionIA_Interact
  (params (ActionValue :type Boolean) (ElapsedSeconds :type Float%20%28double-precision%29) (TriggeredSeconds :type Float%20%28double-precision%29) (InputAction :type Input%20Action%20Object%20Reference :default "/Game/Satisfactory/Blueprints/Inputs/IA_Interact.IA_Interact"))
  (:Started
    (bind (_outhit _returnvalue) (CallFunction|LineTracefromCamera "TraceTypeQuery1"))
    (if _returnvalue
      (if (Utilities|DoesObjectImplementInterface (.HitActor (Collision|BreakHitResult _outhit)) "/Game/Satisfactory/Blueprints/BPI_Interact.BPI_Interact_C")
        (Class|BPIInteract|InteractwithActor(Message) (.HitActor (Collision|BreakHitResult _outhit)) self)))))

(event Input|EnhancedActionEvents|EnhancedInputActionIA_Pause
  (params (ActionValue :type Boolean) (ElapsedSeconds :type Float%20%28double-precision%29) (TriggeredSeconds :type Float%20%28double-precision%29) (InputAction :type Input%20Action%20Object%20Reference :default "/Game/Satisfactory/Blueprints/Inputs/IA_Pause.IA_Pause"))
  (bind _returnvalue (Game|GetPlayerController 0))
  (:Started
    (bind _returnvalue_2 (UserInterface|CreateWidget "/Game/Satisfactory/UI/menus/Pausemenu_WB.Pausemenu_WB_C"))
    (UserInterface|Viewport|AddtoViewport _returnvalue_2 0)
    (Variables|/Script/Engine.PlayerController|SetbShowMouseCursor _returnvalue true)
    (Input|SetInputModeUIOnly _returnvalue 0 "DoNotLock" false)
    (Game|SetGamePaused true)))

(event Input|EnhancedActionEvents|EnhancedInputActionIA_Object2
  (params (ActionValue :type Boolean) (ElapsedSeconds :type Float%20%28double-precision%29) (TriggeredSeconds :type Float%20%28double-precision%29) (InputAction :type Input%20Action%20Object%20Reference :default "/Game/Satisfactory/Blueprints/Inputs/IA_Object2.IA_Object2"))
  (:Started
    (CallFunction|SpawnBuild "/Game/Satisfactory/Blueprints/Buildings/A_Builds_Conveyor.A_Builds_Conveyor_C")))

(event EventBeginPlay
  (|CallParentFunction)
  (Variables|Default|SetCurrentHealth (Variables|Default|GetMaxHealth))
  (Input|AddMappingContext (PlayerController|LocalPlayerSubsystems|GetEnhancedInputLocalPlayerSubsystem (Game|GetPlayerController 0)) "/Game/Satisfactory/Blueprints/Inputs/IMC_Satisfactory.IMC_Satisfactory" 0 "(bIgnoreAllPressedKeysUntilRelease=True,bForceImmediately=False)")
  (CallFunction|CheckCustomDateEvents)
  (bind _asfps_satisfactory_controller (Utilities|Casting|CastToFPS_Satisfactory_Controller (Pawn|GetController)))
  (Default|UpdateHealthBar _asfps_satisfactory_controller (Variables|Default|GetCurrentHealth) (Variables|Default|GetMaxHealth)))

(event Game|Damage|EventAnyDamage
  (params (Damage :type Float%20%28single-precision%29) (DamageType :type Damage%20Type%20Object%20Reference) (InstigatedBy :type Controller%20Object%20Reference) (DamageCauser :type Actor%20Object%20Reference))
  (Variables|Default|SetCurrentHealth (Math|Float|Clamp(Float) (- (Variables|Default|GetCurrentHealth) Damage) 0.0 (Variables|Default|GetMaxHealth)))
  (bind _asfps_satisfactory_controller (Utilities|Casting|CastToFPS_Satisfactory_Controller (Pawn|GetController)))
  (Default|UpdateHealthBar _asfps_satisfactory_controller (Variables|Default|GetCurrentHealth) (Variables|Default|GetMaxHealth))
  (if (<= (Variables|Default|GetCurrentHealth) 0.0)
    (Actor|DestroyActor)))

(event EventOnLanded
  (params (Hit :type Hit%20Result%20Structure%20%28by%20ref%29))
  (CallFunction|Falling))

(event EventDestroyed
  (bind _returnvalue (Game|GetPlayerController 0))
  (if (<= (Variables|Default|GetCurrentHealth) 0.0)
    (bind _returnvalue_2 (UserInterface|CreateWidget "/Game/Satisfactory/UI/menus/WB_PlayerDeath.WB_PlayerDeath_C"))
    (UserInterface|Viewport|AddtoViewport _returnvalue_2 0)
    (Variables|/Script/Engine.PlayerController|SetbShowMouseCursor _returnvalue true)
    (Input|SetInputModeUIOnly _returnvalue 0 "DoNotLock" false)
    (Game|SetGamePaused true)
    (bind _outactors (Actor|GetAllActorsOfClass "/Game/Satisfactory/respawnPos.respawnPos_C"))
    (bind _asrespawn_pos (Utilities|Casting|CastTorespawnPos (Utilities|Array|Get(acopy) _outactors)))
    (bind _asbp_fps_satisfactory_game_mode (Utilities|Casting|CastToBP_FPS_Satisfactory_GameMode (Game|GetGameMode)))
    (Default|RespawnPlayer _asbp_fps_satisfactory_game_mode (Transformation|GetActorTransform _asrespawn_pos))))

(event Input|KeyboardEvents|LeftCtrl
  (params (Key :type Key%20Structure :default "None"))
  (:Pressed
    (Variables|Default|SetIsCtrlDown true))
  (:Released
    (Variables|Default|SetIsCtrlDown false)))

(event Input|KeyboardEvents|LeftShift
  (params (Key :type Key%20Structure :default "None"))
  (:Pressed
    (CallFunction|StartSprinting)
    (Variables|/Script/Engine.CharacterMovementComponent|SetMaxWalkSpeed (Variables|Character|GetCharacterMovement) 1.5e+03))
  (:Released
    (CallFunction|StopSprinting)
    (Variables|/Script/Engine.CharacterMovementComponent|SetMaxWalkSpeed (Variables|Character|GetCharacterMovement) 6e+02)))

(fn ConstructionScript
  (|CallParentFunction))

(fn SpawnBuild
  (params (Class :type A%20Builds%20Object%20Reference))
  (if (Utilities|Time|IsValidTimerHandle (Variables|Default|GetDeleteBuild))
    (Utilities|Time|ClearandInvalidateTimerbyHandle (Variables|Default|GetDeleteBuild)))
  (bind _itemtobuild (Variables|Default|GetItemToBuild)
    (:then
      (Default|CancelBuild _itemtobuild))
    (:else
      _))
  (bind (_outhit _returnvalue) (CallFunction|LineTracefromCamera "TraceTypeQuery4"))
  (if _returnvalue
    (bind _returnvalue_2 (Game|SpawnActorfromClass Class (Math|Transform|MakeTransform (.ImpactPoint (Collision|BreakHitResult _outhit)) (Math|Rotator|MakeRotator (.ImpactPoint (Collision|BreakHitResult _outhit))) "1.000000,1.000000,1.000000") "Undefined" 0 0 0))
    (Variables|Default|SetItemToBuild _returnvalue_2)
    (bind _returnvalue_3 (Utilities|Time|SetTimerbyFunctionName 0 "MovingBuild" 0.05 true))
    (Variables|Default|SetMoveBuild _returnvalue_3)))

(fn MovingBuild
  (bind (_outhit _returnvalue) (CallFunction|LineTracefromCamera "TraceTypeQuery1"))
  (if _returnvalue
    (Default|UpdateLocation (Variables|Default|GetItemToBuild) _outhit)))

(fn PlaceBuild
  (if (.returnValue (Default|IsBuildable (Variables|Default|GetItemToBuild)))
    (bind _returnvalue (Default|PlaceBuild (Variables|Default|GetItemToBuild)))
    (if _returnvalue
      (Utilities|Time|ClearandInvalidateTimerbyHandle (Variables|Default|GetMoveBuild))
      (Variables|Default|SetItemToBuild 0))))

(fn CancleBuild
  (Default|CancelBuild (Variables|Default|GetItemToBuild))
  (Variables|Default|SetItemToBuild 0)
  (Utilities|Time|ClearandInvalidateTimerbyHandle (Variables|Default|GetMoveBuild)))

(fn DeterminDelete
  (bind _outhit (CallFunction|LineTracefromCamera "TraceTypeQuery3"))
  (bind _itemtodelete (Variables|Default|GetItemToDelete)
    (:then
      (if (not (== _itemtodelete (.HitActor (Collision|BreakHitResult _outhit))))
        (Default|SetAllMaterials (Variables|Default|GetItemToDelete) 0 true)
        (bind _asa_builds (Utilities|Casting|CastToA_Builds (.HitActor (Collision|BreakHitResult _outhit)) :!label _label)
          (:then
            (bind _output_get (Variables|Default|SetItemToDelete _asa_builds))
            (Default|SetAllMaterials _output_get "/Game/Satisfactory/Assets/Material/MI_Hologram_Delete.MI_Hologram_Delete" false))
          (:CastFailed
            (bind _output_get_2 (Variables|Default|SetItemToDelete 0))))))
    (:else
      (goto _label))))

(fn LineTracefromCamera
  (params (TraceChannel :type ETraceTypeQuery%20Enum :default "TraceTypeQuery1"))
  (bind _firstpersoncamera (Variables|Default|GetFirstPersonCamera))
  (bind _returnvalue (Transformation|GetWorldLocation _firstpersoncamera))
  (bind (_outhit _returnvalue_2) (Collision|LineTraceByChannel _returnvalue (+ _returnvalue (* (Math|Vector|GetForwardVector _firstpersoncamera) 1500)) TraceChannel false (Utilities|Array|MakeArray 0) "None"))
  (return _outhit _returnvalue_2))

(fn PickupItem
  (params (New%20Item :type A%20Item%20Object%20Reference)))