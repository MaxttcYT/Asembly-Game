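; Game mode for the FPS Satisfactory game, providing an event that respawns the player at a given transform.
; Respawning spawns a new FPS_Satisfactory character, possesses it with player 0's controller, applies one point of damage, then adds one health back and updates the controller's health bar.
; Savegame load-or-create logic for the "savegame" slot is present but never runs, and BeginPlay is empty.
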(event Custom|Respawn%20Player
  (params (SpawnTransform :type Transform))
  (bind _returnvalue (Game|SpawnActorfromClass "/Game/Satisfactory/Blueprints/FPS_Satisfactory.FPS_Satisfactory_C" SpawnTransform "Undefined" 0 0))
  (Pawn|Possess (Game|GetPlayerController 0) _returnvalue)
  (Game|Damage|ApplyDamage _returnvalue 1.0 0 0 "/Script/Engine.DamageType")
  (Utilities|IsValid _returnvalue
    (:Is%20Valid
      (bind _output_get (Variables|/Game/Satisfactory/Blueprints/FPS_Satisfactory.FPS_Satisfactory_C|SetCurrentHealth _returnvalue (+ (Variables|/Game/Satisfactory/Blueprints/FPS_Satisfactory.FPS_Satisfactory_C|GetCurrentHealth _returnvalue) 1.0)))
      (bind _asfps_satisfactory_controller (Utilities|Casting|CastToFPS_Satisfactory_Controller (Pawn|GetController _returnvalue)))
      (Default|UpdateHealthBar _asfps_satisfactory_controller _output_get (Variables|/Game/Satisfactory/Blueprints/FPS_Satisfactory.FPS_Satisfactory_C|GetMaxHealth _returnvalue)))))

(event EventBeginPlay)

(fn ConstructionScript)