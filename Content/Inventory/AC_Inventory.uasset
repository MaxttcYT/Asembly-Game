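; Inventory component that stores item stacks in a slot-keyed map capped at MaxSize, with an input-toggled UMG window.
; The Enhanced Input action creates or removes UMG_Inventory, switches cursor and input mode, and binds the widget's add, drop and remove events.
; PickUpItem tops up matching stacks, then uses an empty slot, respecting MaxStack and AllowDuplicates.
; ItemDropped box-traces downward ahead of the owner to spawn A_Item; HasPlaceForItem checks capacity.
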(event Custom|CE_Default%20Inventory
  (bind _returnvalue (Game|GetPlayerController 0))
  (bind _returnvalue_2 (Game|GetPlayerController 0))
  (Variables|Default|GetAs%20UMG_Inventory
    (:then
      (Variables|/Script/Engine.PlayerController|SetbShowMouseCursor _returnvalue false)
      (Input|SetInputModeGameOnly _returnvalue true)
      (Widget|RemovefromParent (Variables|Default|GetAs%20UMG_Inventory))
      (Variables|Default|SetAs%20UMG_Inventory 0))
    (:else
      (bind _returnvalue_3 (UserInterface|CreateWidget "/Game/Inventory/Widgets/UMG_Inventory.UMG_Inventory_C" 0 (Variables|Default|GetInventory) (Variables|Default|GetMaxSize) (Variables|Default|GetAllowDuplicates) self))
      (bind _output_get (Variables|Default|SetAs%20UMG_Inventory _returnvalue_3))
      (UserInterface|Viewport|AddtoViewport _output_get 0)
      (EventDispatchers|BindEventtoItemAdded (Variables|Default|GetAs%20UMG_Inventory) (EventDispatchers|CreateEvent :!event ItemAdded))
      (EventDispatchers|BindEventtoItemDropped (Variables|Default|GetAs%20UMG_Inventory) (EventDispatchers|CreateEvent :!event ItemDropped))
      (EventDispatchers|BindEventtoItemRemoved (Variables|Default|GetAs%20UMG_Inventory) (EventDispatchers|CreateEvent :!event ItemRemoved))
      (Variables|/Script/Engine.PlayerController|SetbShowMouseCursor _returnvalue_2 true)
      (Input|SetInputModeGameandUI _returnvalue_2 0 "DoNotLock" true false))))

(event Input|EnhancedActionEvents|EnhancedInputActionIA_Inventory
  (params (ActionValue :type Boolean) (ElapsedSeconds :type Float%20%28double-precision%29) (TriggeredSeconds :type Float%20%28double-precision%29) (InputAction :type Input%20Action%20Object%20Reference :default "/Game/Inventory/IA_Inventory.IA_Inventory"))
  (:Started
    (CallFunction|CEDefaultInventory)))

(event EventBeginPlay
  (Input|AddMappingContext (PlayerController|LocalPlayerSubsystems|GetEnhancedInputLocalPlayerSubsystem (Game|GetPlayerController 0)) "/Game/Inventory/IMC_Inventory.IMC_Inventory" 0 "(bIgnoreAllPressedKeysUntilRelease=True,bForceImmediately=False)"))

(fn PickUpItem
  (params (Item :type A%20Item%20Object%20Reference) (Override :type ST%20Inventory%20Structure))
  (bind _structure (Variables|/Game/Satisfactory/Blueprints/A_Item.A_Item_C|GetStructure Item))
  (bind _l_index (LocalVariables|GetL-Index))
  (bind _inventory (Variables|Default|GetInventory))
  (bind _l_index_2 (LocalVariables|GetL-Index))
  (bind (_quantity _itemdata) (Utilities|Struct|BreakST_Inventory _structure))
  (bind (_quantity_2 _itemdata_2) (Utilities|Struct|BreakST_Inventory Override))
  (bind (_returnvalue _remaining) (CallFunction|IsKeyFull _l_index))
  (bind _value (Utilities|Map|Find _inventory _l_index_2))
  (Utilities|IsValid Item
    (:Is%20Valid
      (LocalVariables|SetL-QuantityIn _quantity)
      (LocalVariables|SetL-dataAssetIn _itemdata))
    (:Is%20Not%20Valid
      (LocalVariables|SetL-QuantityIn _quantity_2)
      (LocalVariables|SetL-dataAssetIn _itemdata_2)))
  (while (and (> (LocalVariables|GetL-QuantityIn) 0) (< (LocalVariables|GetL-Index) (Variables|Default|GetMaxSize)))
    (Utilities|FlowControl|Sequence
      (:then_0
        (if _returnvalue
          (if (== (.itemdata (.Value (Utilities|Map|Find (Variables|Default|GetInventory) (LocalVariables|GetL-Index)))) (LocalVariables|GetL-dataAssetIn))
            (LocalVariables|SetL-FoundSameItem true))
          (else
            (bind _output_get (LocalVariables|SetL-Remaining _remaining))
            (if (== _output_get -1)
              (if (== -1 (LocalVariables|GetL-EmptyKey))
                (LocalVariables|SetL-EmptyKey (LocalVariables|GetL-Index)))
              (elif (== (.itemdata _value) (LocalVariables|GetL-dataAssetIn))
                (Utilities|Map|Add (Variables|Default|GetInventory) (LocalVariables|GetL-Index) (Utilities|Struct|MakeST_Inventory (+ (.quantity _value) (Math|Integer|Clamp(Integer) (LocalVariables|GetL-QuantityIn) 0 (LocalVariables|GetL-Remaining))) (LocalVariables|GetL-dataAssetIn)))
                (LocalVariables|SetL-QuantityIn (Math|Integer|Clamp(Integer) (- (LocalVariables|GetL-QuantityIn) (LocalVariables|GetL-Remaining)) 0 (- (LocalVariables|GetL-QuantityIn) (LocalVariables|GetL-Remaining))))
                (LocalVariables|SetL-FoundSameItem true))))))
      (:then_1
        (Math|Integer|IncrementInt (LocalVariables|GetL-Index)))))
  (if (== (LocalVariables|GetL-QuantityIn) 0)
    (return true)
    (elif (and (not (Variables|Default|GetAllowDuplicates)) (LocalVariables|GetL-FoundSameItem))
      (Default|ModifyQuantity Item (LocalVariables|GetL-QuantityIn))
      (return false)
      (else
        ;[1 1 1] Modifications applied
        (if (!= (LocalVariables|GetL-EmptyKey) -1)
          (if (> (Variables|/Game/Satisfactory/Blueprints/Items/DataAsset/DA_Items.DA_Items_C|GetMaxStack (LocalVariables|GetL-dataAssetIn)) (LocalVariables|GetL-QuantityIn))
            ;;[1 1 1] Default Setup
            (Utilities|Map|Add (Variables|Default|GetInventory) (LocalVariables|GetL-EmptyKey) (Utilities|Struct|MakeST_Inventory (LocalVariables|GetL-QuantityIn) (LocalVariables|GetL-dataAssetIn)))
            (return true)
            (else
              ;;[1 1 1] Add a clamped version of the quantity in
              (Utilities|Map|Add (Variables|Default|GetInventory) (LocalVariables|GetL-EmptyKey) (Utilities|Struct|MakeST_Inventory (Math|Integer|Clamp(Integer) (LocalVariables|GetL-QuantityIn) 0 (Variables|/Game/Satisfactory/Blueprints/Items/DataAsset/DA_Items.DA_Items_C|GetMaxStack (LocalVariables|GetL-dataAssetIn))) (LocalVariables|GetL-dataAssetIn)))
              ;;[1 1 1] Modify the quantity of the item as it still has some remaining (leave return false to not destroy item)
              (Default|ModifyQuantity Item (- (LocalVariables|GetL-QuantityIn) (Variables|/Game/Satisfactory/Blueprints/Items/DataAsset/DA_Items.DA_Items_C|GetMaxStack (LocalVariables|GetL-dataAssetIn))))
              (return true)))
          (else
            (return false)))))))

(fn IsKeyFull
  (params (Key :type Integer))
  (bind _inventory (Variables|Default|GetInventory))
  (bind (_value _returnvalue) (Utilities|Map|Find _inventory Key))
  (bind (_quantity _itemdata) (Utilities|Struct|BreakST_Inventory _value))
  (bind _maxstack (Variables|/Game/Satisfactory/Blueprints/Items/DataAsset/DA_Items.DA_Items_C|GetMaxStack _itemdata))
  (bind _returnvalue_2 (- _maxstack _quantity))
  (if _returnvalue
    (return (and (== _returnvalue_2 0) (!= _maxstack 0)) _returnvalue_2)
    (else
      (return false -1))))

(fn ItemAdded
  (params (Slot%20Key :type Integer) (Slot%20Value :type ST%20Inventory%20Structure))
  (Utilities|Map|Add (Variables|Default|GetInventory) Slot%20Key Slot%20Value))

(fn ItemDropped
  (params (ItemDropped :type ST%20Inventory%20Structure))
  (bind _returnvalue (Components|GetOwner))
  (bind _returnvalue_2 (Transformation|GetActorForwardVector _returnvalue))
  (bind _returnvalue_3 (Transformation|GetActorLocation _returnvalue))
  (bind _returnvalue_4 (* _returnvalue_2 3e+02))
  (bind _returnvalue_5 (+ _returnvalue_4 _returnvalue_3))
  (bind (_outhit _returnvalue_6) (Collision|BoxTraceByChannel _returnvalue_5 (- _returnvalue_5 "0.000000,0.000000,500.000000") "15.000000,15.000000,15.000000" "0, 0, 0" "TraceTypeQuery1" false (Utilities|Array|MakeArray (Components|GetOwner)) "None"))
  (if _returnvalue_6
    (Game|SpawnActorfromClass "/Game/Satisfactory/Blueprints/A_Item.A_Item_C" (Math|Transform|MakeTransform (.ImpactPoint (Collision|BreakHitResult _outhit)) "0, 0, 0" "1.000000,1.000000,1.000000") "Undefined" 0 0 1e+02 ItemDropped 0)))

(fn ItemRemoved
  (params (Key :type Integer))
  (Utilities|Map|Remove (Variables|Default|GetInventory) Key))

(fn HasPlaceforItem
  (params (Structure :type ST%20Inventory%20Structure))
  (if (> (Variables|Default|GetMaxSize) (Utilities|Map|Length (Variables|Default|GetInventory)))
    (return true)
    (else
      (bind _output_get (LocalVariables|SetL-QuantityIn (.quantity Structure)))
      (while (and (> _output_get 0) (< (LocalVariables|GetL-Index) (Variables|Default|GetMaxSize)))
        (bind _keys (Utilities|Map|Keys (Variables|Default|GetInventory)))
        (if (== (.itemdata Structure) (.itemdata (.Value (Utilities|Map|Find (Variables|Default|GetInventory) (Utilities|Array|Get(acopy) _keys (LocalVariables|GetL-Index))))))
          (LocalVariables|SetL-QuantityIn (- (LocalVariables|GetL-QuantityIn) (- (Variables|/Game/Satisfactory/Blueprints/Items/DataAsset/DA_Items.DA_Items_C|GetMaxStack (.itemdata (.Value (Utilities|Map|Find (Variables|Default|GetInventory) (Utilities|Array|Get(acopy) _keys (LocalVariables|GetL-Index)))))) (.quantity (.Value (Utilities|Map|Find (Variables|Default|GetInventory) (Utilities|Array|Get(acopy) _keys (LocalVariables|GetL-Index))))))))))
      (return (<= (LocalVariables|GetL-QuantityIn) 0)))))